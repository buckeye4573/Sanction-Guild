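; Game instance that owns save data and UI screens, and opens the first level.
; Display events lazily create, cache and show widgets for menus, HUD, loading and saving messages.
; On Init it synchronously loads the SG_SaveGame slot, or creates a new save object if none exists.
; Player and game-info saves write into that object, sync or async; only async loads fire the loaded dispatcher.
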(event Custom|Display_MessageSaving
  (Variables|SaveGame|GetW_MessageSaving
    (:then
      _)
    (:else
      (bind _returnvalue (UserInterface|CreateWidget "/Game/_Main/Framework/SaveGame/W_MessageSaving.W_MessageSaving_C" (Game|GetPlayerController 0)))
      (bind _output_get (Variables|SaveGame|SetW_MessageSaving _returnvalue))))
  (UserInterface|Viewport|AddtoViewport _output_get 0))

(event Custom|Display_LoadingScreen
  ;[0.15 0.15 0.15 0.5] Display HUD
  (Variables|Default|GetW_ScreenLoading
    (:then
      _)
    (:else
      (bind _returnvalue (UserInterface|CreateWidget "/Game/_Main/UI/Screen_Loading/W_ScreenLoading.W_ScreenLoading_C" (Game|GetPlayerController 0)))
      (bind _output_get (Variables|Default|SetW_ScreenLoading _returnvalue))))
  (UserInterface|Viewport|AddtoViewport _output_get 0))

(event Custom|Display_SinglePlayer
  ;[0.15 0.15 0.15 0.5] Single Player
  (Variables|MainMenu|GetW_SinglePlayer
    (:then
      _)
    (:else
      (bind _returnvalue (UserInterface|CreateWidget "/Game/_Main/Levels/MainMenu/UI/W_SinglePlayer.W_SinglePlayer_C" (Game|GetPlayerController 0)))
      (bind _output_get (Variables|MainMenu|SetW_SinglePlayer _returnvalue))))
  (UserInterface|Viewport|AddtoViewport _output_get 0))

(event Custom|Display_MainMenu
  ;[0.15 0.15 0.15 0.5] Main Menu
  (Variables|MainMenu|GetW_MainMenu
    (:then
      _)
    (:else
      (bind _returnvalue (UserInterface|CreateWidget "/Game/_Main/Levels/MainMenu/UI/W_MainMenu.W_MainMenu_C" (Game|GetPlayerController 0)))
      (bind _output_get (Variables|MainMenu|SetW_MainMenu _returnvalue))))
  (UserInterface|Viewport|AddtoViewport _output_get 0)
  (Variables|/Script/Engine.PlayerController|SetbShowMouseCursor (Game|GetPlayerController 0) true))

(event Custom|Display_HUD
  ;[0.15 0.15 0.15 0.5] Display HUD
  (Variables|UI|GetW_HUD
    (:then
      _)
    (:else
      (bind _returnvalue (UserInterface|CreateWidget "/Game/_Main/UI/HUD/W_HUD.W_HUD_C" (Game|GetPlayerController 0)))
      (bind _output_get (Variables|UI|SetW_HUD _returnvalue))))
  (UserInterface|Viewport|AddtoViewport _output_get 0))

(event Custom|OpenLevel
  (Game|OpenLevel(byName) "Map_Level01"))

(event Custom|CreateSaveGame
  (bind _returnvalue (SaveGame|CreateSaveGameObject "/Game/_Main/Framework/SaveGame/SG_SaveGame.SG_SaveGame_C"))
  (Variables|SaveGame|SetSavedGameData _returnvalue))

(event EventSaveGameData
  (params (Async :type Boolean))
  ;[0.15 0.15 0.15 0.5] Save Game Data
  (if Async
    (|AsyncSaveGametoSlot (Variables|SaveGame|GetSavedGameData) (Variables|SaveGame|GetSlotName))
    (else
      (SaveGame|SaveGametoSlot (Variables|SaveGame|GetSavedGameData) (Variables|SaveGame|GetSlotName)))))

(event EventLoadGame
  (params (Async :type Boolean))
  (bind _slotname (Variables|SaveGame|GetSlotName))
  ;[0.15 0.15 0.15 0.5] Load Game
  (bind _returnvalue (SaveGame|DoesSaveGameExist (Variables|SaveGame|GetSlotName)))
  (if _returnvalue
    (if Async
      (bind _savegame (|AsyncLoadGamefromSlot _slotname)
        (:Completed
          (bind _assg_save_game (Utilities|Casting|CastToSG_SaveGame _savegame))
          (Variables|SaveGame|SetSavedGameData _assg_save_game)
          (Default|CallEDonGameLoaded)))
      (else
        (bind _returnvalue_2 (SaveGame|LoadGamefromSlot _slotname))
        (bind _assg_save_game_2 (Utilities|Casting|CastToSG_SaveGame _returnvalue_2))
        (Variables|SaveGame|SetSavedGameData _assg_save_game_2)))
    (else
      (CallFunction|CreateSaveGame))))

(event EventSavePlayer
  (params (PlayerSave :type S%20Player%20Save%20Structure) (Async :type Boolean))
  ;[0.15 0.15 0.15 0.5] Player Save
  (Variables|/Game/_Main/Framework/SaveGame/SG_SaveGame.SG_SaveGame_C|SetPlayerSave (Variables|SaveGame|GetSavedGameData) PlayerSave)
  (CallFunction|SaveGameData Async))

(event EventSaveGameInfo
  (params (GameInfoSave :type S%20Save%20Game%20Info%20Structure) (Async :type Boolean))
  ;[0.15 0.15 0.15 0.5] Save Game Info
  (Variables|/Game/_Main/Framework/SaveGame/SG_SaveGame.SG_SaveGame_C|SetSaveGameInfo (Variables|SaveGame|GetSavedGameData) GameInfoSave)
  (CallFunction|SaveGameData Async))

(event EventInit
  (CallFunction|LoadGame false))

(fn GetGameData
  (bind _savedgamedata (Variables|SaveGame|GetSavedGameData))
  (Development|PrintString (Utilities|GetDisplayName _savedgamedata) true true "(R=0.000000,G=0.660000,B=1.000000,A=1.000000)" 1e+01)
  (return _savedgamedata))

(fn NewGI
  (return self))
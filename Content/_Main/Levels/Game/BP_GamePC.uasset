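; BP_GamePC is the in-game player controller that sets up the HUD and passes health values to it.
; On BeginPlay it clears all widgets, caches the game instance returned by NewGIMessage and has it display the HUD.
; Attribute events relay current and maximum health to the HUD's attributes widget through that cached reference.
; It also exposes itself through a GamePC getter and quits the game on a debug Escape key.
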(event EventBeginPlay
  ;[0.15 0.15 0.15 0.5] Begin Play
  (Viewport|RemoveAllWidgets)
  (bind _newgi (Class|BPINewGI|NewGI(Message) (Game|GetGameInstance)))
  (bind _output_get (Variables|Framework|SetNew%20GI _newgi))
  (Default|DisplayHUD _output_get))

(event Input|KeyboardEvents|DebugKeyEscape
  (params (Key :type Key%20Structure :default "None") (ActionValue :type Input%20Action%20Value%20Structure))
  (:Pressed
    (Game|QuitGame 0 "Quit" false)))

(event Custom|Update_Attributes_PC
  (params (CurrentHealth :type Float%20%28double-precision%29) (MaxHealth :type Float%20%28double-precision%29))
  (Default|UpdateHealth (Variables|/Game/_Main/UI/HUD/W_HUD.W_HUD_C|GetW_Attributes (Variables|/Game/_Main/Framework/BP_NewGI.BP_NewGI_C|GetW_HUD (Variables|Framework|GetNew%20GI))) CurrentHealth MaxHealth))

(event Custom|PC_Attributes
  (params (CurrentHealth :type Float%20%28double-precision%29) (MaxHealth :type Float%20%28double-precision%29))
  (CallFunction|UpdateAttributesPC CurrentHealth MaxHealth))

(fn ConstructionScript)

(fn GamePC
  (return self))
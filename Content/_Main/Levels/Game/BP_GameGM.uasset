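; Game mode for a multiplayer level that tracks player controllers and runs a shared start countdown.
; PostLogin gets each controller through a GamePCMessage call and adds it to AllConnectedPlayers.
; Countdown uses a Started flag to show the timer on all controllers once, then calls unfreeze after a fixed delay.
; Freeze and unfreeze events loop over the player list, and a GameGM getter returns the mode itself.
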(event Custom|Client_Unfreeze
  (for _array_element (Variables|Default|GetAllConnectedPlayers)
    (Default|ClientUnfreeze _array_element)))

(event Custom|Client_Freeze
  (for _array_element (Variables|Default|GetAllConnectedPlayers)
    (Default|ClientFreeze _array_element)))

(event Custom|Countdown
  (for _array_element (Variables|Default|GetAllConnectedPlayers)
    (if (not (Variables|Default|GetStarted?))
      (for _array_element_2 (Variables|Default|GetAllConnectedPlayers)
        (Default|ShowCountdown _array_element_2))
      (Variables|Default|SetStarted? true)
      (Utilities|FlowControl|Delay 1e+01)
      (CallFunction|ClientUnfreeze))))

(event EventBeginPlay)

(event EventPostLogin
  (params (NewPlayer :type Player%20Controller%20Object%20Reference))
  ;[0.15 0.15 0.15 0.5] Event On Post Login
  (bind _gamepc (Class|BPIGamePC|GamePC(Message) NewPlayer))
  (bind _output_get (Variables|Default|SetGame%20PC _gamepc))
  (Utilities|Array|Add (Variables|Default|GetAllConnectedPlayers) _output_get))

(fn ConstructionScript)

(fn GameGM
  (return self))
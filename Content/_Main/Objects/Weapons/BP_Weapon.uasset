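; Weapon object that can be interacted with, removing itself from the world after running the parent's interaction logic.
; It reports a fixed interaction type and looks up its stats by row name in DT_Weapons, storing them in SWeaponInfo.
; A pair of Multi_ events switches its RotatingMovement spin on and off.
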(event Custom|Multi_StartWeaponRotation
  ;[0.15 0.15 0.15 0.5] Weapon Rotation
  (Components|Activation|SetActive (Variables|Default|GetRotatingMovement) true false))

(event Custom|Multi_StopWeaponRotation
  ;[0.15 0.15 0.15 0.5] Weapon Rotation
  (Components|Activation|SetActive (Variables|Default|GetRotatingMovement) false false))

(event Custom|SRV_WeaponData
  (params (RowName :type Name))
  ;[0.15 0.15 0.15 0.5] SRV_WeaponData
  (bind _returnvalue (Utilities|GetDataTableRow "/Game/_Main/Objects/Weapons/DT_Weapons.DT_Weapons" RowName)
    (:then
      (Variables|Default|SetS_WeaponInfo _returnvalue))))

(event EventBeginPlay
  (|CallParentFunction))

(event Collision|EventActorBeginOverlap
  (params (OtherActor :type Actor%20Object%20Reference))
  (|CallParentFunction OtherActor))

(event EventTick
  (params (DeltaSeconds :type Float%20%28single-precision%29))
  (|CallParentFunction DeltaSeconds) ; This node is disabled and will not be called.\nDrag off pins to build functionality.
)

(event EventInteract
  (params (Interactor :type BP%20Character%20Combat%20Base%20Object%20Reference))
  ;[0.15 0.15 0.15 0.5] Interact
  (|CallParentFunction Interactor)
  (CallFunction|RemovefromWorld))

(fn ConstructionScript
  (|CallParentFunction))

(fn GetInteractionType
  (return "NewEnumerator4"))
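; BP_Spawner_NonWeapon is a pickup spawner that places a random health or armor pickup at its location.
; On BeginPlay a server-prefixed event sets the object pool component's pooled class, with health weighted two to one over armor.
; After a short delay, the pool component spawns that pickup at the Scene component's world transform.
; The spawn runs once, with no respawn logic in this Blueprint.
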(event Custom|SRV_RandomizeObject
  ;[0.15 0.15 0.15 0.5] Randomize Object
  (Variables|/Game/_Main/Patterns/Pool/BPC_ObjectPool.BPC_ObjectPool_C|SetPooledActorClass (Variables|Default|GetBPC_ObjectPool) (Utilities|Select :Index (Math|Random|RandomIntegerinRange 0 2) :Option%200 "/Game/_Main/Objects/NonWeapons/BP_Pickup_Health.BP_Pickup_Health_C" :Option%201 "/Game/_Main/Objects/NonWeapons/BP_Pickup_Armor.BP_Pickup_Armor_C" :Option%202 "/Game/_Main/Objects/NonWeapons/BP_Pickup_Health.BP_Pickup_Health_C")))

(event EventBeginPlay
  ;[0.15 0.15 0.15 0.5] Event Begin Play
  (CallFunction|SRVRandomizeObject)
  (Utilities|FlowControl|Delay 0.2)
  (Default|FSpawnfromPool (Variables|Default|GetBPC_ObjectPool) (Transformation|GetWorldTransform (Variables|Default|GetScene))))

(fn ConstructionScript)
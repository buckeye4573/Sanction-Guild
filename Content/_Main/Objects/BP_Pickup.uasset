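; BP_Pickup is a bare pickup actor that exposes functions for interaction and collection.
; The interaction getters return fixed defaults: the first enum interaction type, no hold time, no taps and a zero location.
; Pickup returns the actor itself, and the RemoveFromWorld event destroys it.
; SoundEffect is an empty stub, and BeginPlay and construction do nothing.
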(event Custom|RemoveFromWorld
  (Actor|DestroyActor))

(event EventBeginPlay)

(fn ConstructionScript)

(fn GetHoldDuration
  (return 0.0))

(fn GetInteractionType
  (return "NewEnumerator0"))

(fn GetInteractLocation
  (return "0, 0, 0"))

(fn GetTapCount
  (return 0))

(fn Pickup
  (return self))

(fn SoundEffect
  (return 0))
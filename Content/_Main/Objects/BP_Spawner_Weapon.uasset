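; BP_Spawner_Weapon is a placed spawner, named for weapons, that spawns from an object pool.
; On BeginPlay it passes its Scene component's world transform to the BPCObjectPool component's FSpawnFromPool.
; SpawnItem (direct spawn of ItemClass) and StoreArrays (unique transform recording) remain as custom events, but their calls in this graph are disconnected.
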(event Custom|SpawnItem
  ;[0.15 0.15 0.15 0.5] Spawn Item
  (bind _returnvalue (Game|SpawnActorfromClass (Variables|Default|GetItemClass) (Transformation|GetActorTransform) "AdjustIfPossibleButAlwaysSpawn" "MultiplyWithRoot" 0 5.0 0))
  (Variables|Default|SetSpawnedItem _returnvalue))

(event Custom|StoreArrays
  ;[0.15 0.15 0.15 0.5] SRV Store Arrays
  (Utilities|Array|AddUnique (Variables|Default|GetTransformArrays) (Transformation|GetActorTransform)))

(event EventBeginPlay
  (Default|FSpawnfromPool (Variables|Default|GetBPC_ObjectPool) (Transformation|GetWorldTransform (Variables|Default|GetScene))))

(fn ConstructionScript)
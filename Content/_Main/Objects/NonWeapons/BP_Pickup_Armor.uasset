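; Armor pickup that restores armor to the interacting combat character.
; On Interact it reads the character's damage system component and, only if armor is below max, increases it by the pickup's Armor value.
; After a successful pickup it removes itself from the world and triggers a server-side respawn of the object.
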(event EventBeginPlay
  (|CallParentFunction) ; This node is disabled and will not be called.\nDrag off pins to build functionality.
)

(event Collision|EventActorBeginOverlap
  (params (OtherActor :type Actor%20Object%20Reference))
  (|CallParentFunction OtherActor) ; This node is disabled and will not be called.\nDrag off pins to build functionality.
)

(event EventTick
  (params (DeltaSeconds :type Float%20%28single-precision%29))
  (|CallParentFunction DeltaSeconds) ; This node is disabled and will not be called.\nDrag off pins to build functionality.
)

(event EventInteract
  (params (Interactor :type BP%20Character%20Combat%20Base%20Object%20Reference))
  (|CallParentFunction Interactor)
  (bind (_toomuchhealth_ _bpc_damagesystem) (CallFunction|FCheckArmorAmounnt Interactor))
  (if (not _toomuchhealth_)
    (Default|FIncreaseArmor _bpc_damagesystem (Variables|Default|GetArmor))
    (CallFunction|RemovefromWorld)
    (CallFunction|SRVRespawnObject)))

(fn ConstructionScript
  (|CallParentFunction))

(fn GetInteractionType
  (return "NewEnumerator0"))

(fn FCheckArmorAmounnt
  (params (CharacterCombatBase :type BP%20Character%20Combat%20Base%20Object%20Reference))
  (bind _bpc_damagesystem (Variables|/Game/_Main/Characters/BP_Character_Combat_Base.BP_Character_Combat_Base_C|GetBPC_DamageSystem CharacterCombatBase))
  (return (>= (Variables|/Game/_Main/Components/BPC_DamageSystem.BPC_DamageSystem_C|GetCurrentArmor _bpc_damagesystem) (Variables|/Game/_Main/Components/BPC_DamageSystem.BPC_DamageSystem_C|GetMaxArmor _bpc_damagesystem)) _bpc_damagesystem))
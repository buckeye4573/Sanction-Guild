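; Interactable door that swings a mesh around its yaw axis, using a two-second hold duration and the doorknob as interaction point.
; Interact plays a click sound and calls a server event, which toggles open state and multicasts a forward or reversed timeline.
; CanOpen blocks re-triggering until a short delay, started from the timeline update, restores it.
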(event Custom|MC_OpenDoor
  ;[0.15 0.15 0.15 0.5] Open_Close Door
  (bind _zrotation (Timeline|Open%20Door%20Timeline PlayFromStart)
    (:Update
      (bind _staticmesh (Variables|Default|GetStaticMesh)
        (:then
          (Transformation|SetRelativeRotation _staticmesh (Math|Rotator|MakeRotator 0.0 0.0 _zrotation) false false)
          (Utilities|FlowControl|Delay 0.7)
          (Variables|Default|SetCanOpen? true))
        (:else)))))

(event Custom|MC_CloseDoor
  ;[0.15 0.15 0.15 0.5] Open_Close Door
  (bind _zrotation (Timeline|Open%20Door%20Timeline ReverseFromEnd)
    (:Update
      (bind _staticmesh (Variables|Default|GetStaticMesh)
        (:then
          (Transformation|SetRelativeRotation _staticmesh (Math|Rotator|MakeRotator 0.0 0.0 _zrotation) false false)
          (Utilities|FlowControl|Delay 0.7)
          (Variables|Default|SetCanOpen? true))
        (:else)))))

(event Custom|SRV_Interact
  ;[0.15 0.15 0.15 0.5] SRV Interact
  (if (Variables|Default|GetCanOpen?)
    (Variables|Default|SetCanOpen? false)
    (if (not (Variables|Default|GetIsOpen?))
      (Variables|Default|SetIsOpen? true)
      (CallFunction|MCOpenDoor)
      (else
        (Variables|Default|SetIsOpen? false)
        (CallFunction|MCCloseDoor)))))

(event Custom|DoorSound
  (Audio|PlaySoundatLocation "/Engine/VREditor/Sounds/UI/Click_on_Button.Click_on_Button" (Transformation|GetActorLocation) "0, 0, 0" 1.0 1.0 0.0 0 0 self 0))

(event EventInteract
  (params (Interactor :type Actor%20Object%20Reference))
  ;[0.15 0.15 0.15 0.5] Event Interact
  (|CallParentFunction 0)
  (CallFunction|SRVInteract)
  (CallFunction|DoorSound))

(fn ConstructionScript
  (|CallParentFunction))

(fn GetHoldDuration
  (return 2.0))

(fn GetInteractLocation
  (return (Transformation|GetWorldLocation (Variables|Default|GetDoorknob))))
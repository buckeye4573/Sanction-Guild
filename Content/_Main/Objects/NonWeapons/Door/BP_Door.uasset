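; BP_Door is a door object that exposes an interaction interface, but its Interact event is empty, so it has no behavior yet.
; Getter functions report a fixed interaction type, a hold duration read from the Duration variable, and a constant tap count.
; The default BeginPlay, overlap and Tick events are disabled, and the construction script only calls its parent.
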(event EventBeginPlay
  (|CallParentFunction) ; This node is disabled and will not be called.\nDrag off pins to build functionality.
)

(event Collision|EventActorBeginOverlap
  (params (OtherActor :type Actor%20Object%20Reference))
  (|CallParentFunction OtherActor) ; This node is disabled and will not be called.\nDrag off pins to build functionality.
)

(event EventTick
  (params (DeltaSeconds :type Float%20%28single-precision%29))
  (|CallParentFunction DeltaSeconds) ; This node is disabled and will not be called.\nDrag off pins to build functionality.
)

(event EventInteract
  (params (Interactor :type BP%20Character%20Combat%20Base%20Object%20Reference)))

(fn ConstructionScript
  (|CallParentFunction))

(fn GetInteractionType
  (return "NewEnumerator1"))

(fn GetHoldDuration
  (return (Variables|Default|GetDuration)))

(fn GetTapCount
  (return 3))
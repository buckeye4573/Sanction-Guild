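; BP_Pickup_Health is an interactable health pickup that heals the character that uses it.
; On Interact, a helper checks whether the interactor's health component is already at or above max health.
; If not, it calls a server heal on that component with the Healing amount, removes the pickup from the world and triggers a server respawn.
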(event EventBeginPlay
  (|CallParentFunction) ; This node is disabled and will not be called.\nDrag off pins to build functionality.
)

(event Collision|EventActorBeginOverlap
  (params (OtherActor :type Actor%20Object%20Reference))
  (|CallParentFunction OtherActor) ; This node is disabled and will not be called.\nDrag off pins to build functionality.
)

(event EventTick
  (params (DeltaSeconds :type Float%20%28single-precision%29))
  (|CallParentFunction DeltaSeconds) ; This node is disabled and will not be called.\nDrag off pins to build functionality.
)

(event EventInteract
  (params (Interactor :type BP%20Character%20Combat%20Base%20Object%20Reference))
  (|CallParentFunction Interactor)
  (bind (_toomuchhealth_ _bpc_health) (CallFunction|FCheckHealthAmounnt Interactor))
  (if (not _toomuchhealth_)
    (Default|SRVIncreaseHealth _bpc_health (Variables|Default|GetHealing))
    (CallFunction|RemovefromWorld)
    (CallFunction|SRVRespawnObject)))

(fn ConstructionScript
  (|CallParentFunction))

(fn GetInteractionType
  (return "NewEnumerator0"))

(fn FCheckHealthAmounnt
  (params (CharacterCombatBase :type BP%20Character%20Combat%20Base%20Object%20Reference))
  (bind _bpc_health (Variables|/Game/_Main/Characters/BP_Character_Combat_Base.BP_Character_Combat_Base_C|GetBPC_Health CharacterCombatBase))
  (return (>= (Variables|/Game/_Main/Components/BPC_Health.BPC_Health_C|GetCurrentHealth _bpc_health) (Variables|/Game/_Main/Components/BPC_Health.BPC_Health_C|GetMaxHealth _bpc_health)) _bpc_health))
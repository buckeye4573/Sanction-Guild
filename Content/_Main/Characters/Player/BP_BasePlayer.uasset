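; Base player character that handles Enhanced Input movement and look, weapon equipping and firing effects, and saved-position restoring.
; On BeginPlay it adds the input mapping and applies the game instance's saved transform and control rotation, skipping default transforms.
; Damage component health and armor updates, plus missing-weapon messages, are forwarded to the player controller.
; Debug keys trigger loading, saving and test damage.
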(event EventBeginPlay
  ;[0.15 0.15 0.15 0.5] Event Begin Play
  (|CallParentFunction)
  (CallFunction|EventMapping)
  (bind _savegamedata (Class|BPISaveGame|GetGameData(Message) (Game|GetGameInstance)))
  (Utilities|IsValid _savegamedata
    (:Is%20Valid
      (CallFunction|FUsePlayerSave (Variables|/Game/_Main/Framework/SaveGame/SG_SaveGame.SG_SaveGame_C|GetPlayerSave _savegamedata)))))

(event EventMessageBox
  (params (Message :type Text))
  ;[0.15 0.15 0.15 0.5] Message Box
  (bind _game_pc (Variables|Default|GetGame%20PC)
    (:then
      (Default|MessageBox _game_pc Message))
    (:else)))

(event Input|KeyboardEvents|DebugKeyG
  (params (Key :type Key%20Structure :default "None") (ActionValue :type Input%20Action%20Value%20Structure))
  (bind _returnvalue (Game|GetGameInstance))
  (:Pressed
    (Class|BPISaveGame|LoadGame(Message) _returnvalue false)
    (bind _savegamedata (Class|BPISaveGame|GetGameData(Message) _returnvalue))
    (CallFunction|FUsePlayerSave (Variables|/Game/_Main/Framework/SaveGame/SG_SaveGame.SG_SaveGame_C|GetPlayerSave _savegamedata))))

(event Input|KeyboardEvents|DebugKeyU
  (params (Key :type Key%20Structure :default "None") (ActionValue :type Input%20Action%20Value%20Structure))
  (:Pressed
    (bind _playersave (CallFunction|FGetPlayerSave))
    (Class|BPISaveGame|SavePlayer(Message) (Game|GetGameInstance) _playersave false)))

(event Custom|EventMapping
  ;[0.15 0.15 0.15 0.5] Event Mapping
  (bind _asplayer_controller (Utilities|Casting|CastToPlayerController (Pawn|GetController)))
  (Utilities|IsValid (PlayerController|LocalPlayerSubsystems|GetEnhancedInputLocalPlayerSubsystem _asplayer_controller)
    (:Is%20Valid
      (Input|AddMappingContext (PlayerController|LocalPlayerSubsystems|GetEnhancedInputLocalPlayerSubsystem _asplayer_controller) "/Game/_Main/Characters/Player/Inputs/IMC_Player.IMC_Player" 0 "(bIgnoreAllPressedKeysUntilRelease=True,bForceImmediately=False,bNotifyUserSettings=False)"))))

(event Input|EnhancedActionEvents|EnhancedInputActionIA_Move
  (params (ActionValue :type Vector%202D%20Structure) (ElapsedSeconds :type Float%20%28double-precision%29) (TriggeredSeconds :type Float%20%28double-precision%29) (InputAction :type Input%20Action%20Object%20Reference :default "/Game/_Main/Characters/Player/Inputs/InputActions/IA_Move.IA_Move"))
  (bind _returnvalue (Pawn|GetControlRotation :!class /Script/Engine.Pawn))
  ;[0.15 0.15 0.15 0.5] IA Move
  (Pawn|Input|AddMovementInput (Math|Vector|GetRightVector (Math|Rotator|MakeRotator (.roll _returnvalue) 0.0 (.yaw _returnvalue))) (.x ActionValue) false)
  (Pawn|Input|AddMovementInput (Math|Vector|GetForwardVector (Math|Rotator|MakeRotator 0.0 0.0 (.yaw (Pawn|GetControlRotation :!class /Script/Engine.Pawn)))) (.y ActionValue) false))

(event Input|EnhancedActionEvents|EnhancedInputActionIA_MouseLook
  (params (ActionValue :type Vector%202D%20Structure) (ElapsedSeconds :type Float%20%28double-precision%29) (TriggeredSeconds :type Float%20%28double-precision%29) (InputAction :type Input%20Action%20Object%20Reference :default "/Game/_Main/Characters/Player/Inputs/InputActions/IA_MouseLook.IA_MouseLook"))
  ;[0.15 0.15 0.15 0.5] IA MouseLook
  (Pawn|Input|AddControllerYawInput (.x ActionValue))
  (Pawn|Input|AddControllerPitchInput (.y ActionValue)))

(event Input|EnhancedActionEvents|EnhancedInputActionIA_Jump
  (params (ActionValue :type Boolean) (ElapsedSeconds :type Float%20%28double-precision%29) (TriggeredSeconds :type Float%20%28double-precision%29) (InputAction :type Input%20Action%20Object%20Reference :default "/Game/_Main/Characters/Player/Inputs/InputActions/IA_Jump.IA_Jump"))
  ;[0.15 0.15 0.15 0.5] IA Jump
  (:Started
    (Character|Jump))
  (:Canceled
    (Character|StopJumping :!label _label))
  (:Completed
    (goto _label)))

(event Input|EnhancedActionEvents|EnhancedInputActionIA_Crouch
  (params (ActionValue :type Boolean) (ElapsedSeconds :type Float%20%28double-precision%29) (TriggeredSeconds :type Float%20%28double-precision%29) (InputAction :type Input%20Action%20Object%20Reference :default "/Game/_Main/Characters/Player/Inputs/InputActions/IA_Crouch.IA_Crouch"))
  ;[0.15 0.15 0.15 0.5] IA Crouch
  (:Started
    (Character|Crouch))
  (:Canceled
    (Character|UnCrouch :!label _label))
  (:Completed
    (goto _label)))

(event EDUpdateHealth(BPC_DamageSystem)
  (params (CurrentHealth :type Float%20%28double-precision%29) (MaxHealth :type Float%20%28double-precision%29))
  ;[0.15 0.15 0.15 0.5] Health
  (CallFunction|SendAttributestoPC CurrentHealth MaxHealth))

(event EDUpdateArmor(BPC_DamageSystem)
  (params (CurrentArmor :type Float%20%28double-precision%29) (MaxArmor :type Float%20%28double-precision%29))
  ;[0.15 0.15 0.15 0.5] Armor
  (CallFunction|SendArmortoPC CurrentArmor MaxArmor))

(event Custom|SendArmorToPC
  (params (CurrentArmor :type Float%20%28double-precision%29) (MaxArmor :type Float%20%28double-precision%29))
  ;[0.15 0.15 0.15 0.5] Armor
  (bind _game_pc (Variables|Default|GetGame%20PC)
    (:then
      (Default|PCArmor _game_pc CurrentArmor MaxArmor))
    (:else)))

(event Custom|SendAttributestoPC
  (params (CurrentHealth :type Float%20%28double-precision%29) (MaxHealth :type Float%20%28double-precision%29))
  ;[0.15 0.15 0.15 0.5] Health
  (bind _game_pc (Variables|Default|GetGame%20PC)
    (:then
      (Default|PCHealth _game_pc CurrentHealth MaxHealth))
    (:else)))

(event Input|KeyboardEvents|DebugKeyY
  (params (Key :type Key%20Structure :default "None") (ActionValue :type Input%20Action%20Value%20Structure)))

(event Input|KeyboardEvents|DebugKeyT
  (params (Key :type Key%20Structure :default "None") (ActionValue :type Input%20Action%20Value%20Structure))
  (:Pressed
    (Default|SRVDecreaseHealth (Variables|Default|GetBPC_DamageSystem) 1e+01)))

(event Input|EnhancedActionEvents|EnhancedInputActionIA_PrimaryWeapon
  (params (ActionValue :type Boolean) (ElapsedSeconds :type Float%20%28double-precision%29) (TriggeredSeconds :type Float%20%28double-precision%29) (InputAction :type Input%20Action%20Object%20Reference :default "/Game/_Main/Characters/Player/Inputs/InputActions/IA_PrimaryWeapon.IA_PrimaryWeapon"))
  ;[0.15 0.15 0.15 0.5] IA_PrimaryWeapon
  (:Started
    (Variables|Default|GetPrimaryWeaponBase
      (:then
        (CallFunction|SRVEquipPrimary))
      (:else
        (CallFunction|MessageBox "You need a Primary Weapon")))))

(event Input|EnhancedActionEvents|EnhancedInputActionIA_SecondaryWeapon
  (params (ActionValue :type Boolean) (ElapsedSeconds :type Float%20%28double-precision%29) (TriggeredSeconds :type Float%20%28double-precision%29) (InputAction :type Input%20Action%20Object%20Reference :default "/Game/_Main/Characters/Player/Inputs/InputActions/IA_SecondaryWeapon.IA_SecondaryWeapon"))
  ;[0.15 0.15 0.15 0.5] IA_SecondaryWeapon
  (:Started
    (Variables|Default|GetSecondaryWeaponBase
      (:then
        (CallFunction|SRVEquipSecondary))
      (:else
        (CallFunction|MessageBox "You need a Secondary Weapon")))))

(event Input|EnhancedActionEvents|EnhancedInputActionIA_MeleeWeapon
  (params (ActionValue :type Boolean) (ElapsedSeconds :type Float%20%28double-precision%29) (TriggeredSeconds :type Float%20%28double-precision%29) (InputAction :type Input%20Action%20Object%20Reference :default "/Game/_Main/Characters/Player/Inputs/InputActions/IA_MeleeWeapon.IA_MeleeWeapon"))
  ;[0.15 0.15 0.15 0.5] IA_MeleeWeapon
  (:Started
    (CallFunction|SRVNoWeapons)))

(event Input|EnhancedActionEvents|EnhancedInputActionIA_UseWeapon
  (params (ActionValue :type Boolean) (ElapsedSeconds :type Float%20%28double-precision%29) (TriggeredSeconds :type Float%20%28double-precision%29) (InputAction :type Input%20Action%20Object%20Reference :default "/Game/_Main/Characters/Player/Inputs/InputActions/IA_UseWeapon.IA_UseWeapon"))
  (bind _weaponinfo (Variables|Default|GetWeaponInfo))
  (bind (_sound_fire _muzzleflash _muzzlesocket) (Utilities|Struct|BreakS_WeaponInfo _weaponinfo))
  ;[0.15 0.15 0.15 0.5] IA_UseWeapon
  (:Started
    (bind _weaponbase (Variables|Default|GetWeaponBase)
      (:then
        (Default|MCWeaponEffects _weaponbase _muzzleflash _muzzlesocket _sound_fire (.location (Transformation|GetActorTransform))))
      (:else))))

(fn ConstructionScript
  (|CallParentFunction))

(fn FGetPlayerSave
  (return (Utilities|Struct|MakeS_PlayerSave (Transformation|GetActorTransform) (Pawn|GetControlRotation :!class /Script/Engine.Pawn))))

(fn FUsePlayerSave
  (params (PlayerSave :type S%20Player%20Save%20Structure))
  (if (not (== (.transform PlayerSave) (Math|Transform|MakeTransform "0, 0, 0")))
    (Transformation|SetActorTransform (.transform PlayerSave))
    (Pawn|SetControlRotation (Pawn|GetController) (.controlrotation PlayerSave))
    (return)))

(fn BasePlayer
  (return self))
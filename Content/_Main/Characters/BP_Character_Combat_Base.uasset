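; Base combat character that handles primary and secondary weapon ownership and exposes health, healing and damage through BPC_DamageSystem.
; After a short delay the authority initializes the interact, base and damage components.
; Equip interactions route to SRV events that spawn weapons from DT_Weapons, then MC events attach them to mesh sockets and send the combat blendspace to the AnimInstance.
; Death, block and damage-response handlers are bound in construction but left empty.
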(event OnInteraction(BPC_Interact)
  (params (Equip :type BP%20Pickup%20Object%20Reference))
  ;[0.15 0.15 0.15 0.5] On Interaction
  (bind _output_get (Variables|Default|SetPickup Equip))
  (bind _interactiontype (Class|BPIInteractable|GetInteractionType(Message) _output_get))
  (Default|Interact _output_get self)
  (switch Utilities|FlowControl|Switch|SwitchonE_InteractionType _interactiontype
    (:NewEnumerator4
      (CallFunction|FOwnWeapon (Variables|/Game/_Main/Objects/BP_Pickup.BP_Pickup_C|GetActiveWeapon _output_get) (Variables|/Game/_Main/Objects/BP_Pickup.BP_Pickup_C|GetRowName _output_get)))))

(event EventBeginPlay
  ;[0.15 0.15 0.15 0.5] Event Begin Play
  (|CallParentFunction)
  (bind _gamepc (Class|BPIGamePC|GamePC(Message) (Game|GetPlayerController 0)))
  (Variables|Default|SetGame%20PC _gamepc)
  (Networking|SwitchHasAuthority
    (:Authority
      (Utilities|FlowControl|Delay 1.5)
      (Default|Initialize (Variables|Default|GetBPC_Interact)))))

(event Custom|MC_CombatState
  (params (Blendspace :type Integer))
  ;[0.15 0.15 0.15 0.5] MC Combat State
  (Class|BPIAnimBPPlayer|CombatState(Message) (Components|SkeletalMesh|GetAnimInstance (Variables|Character|GetMesh)) Blendspace))

(event Custom|Death
  (params (Character :type Actor%20Object%20Reference)))

(event Custom|Blocked
  (params (CanBeParried? :type Boolean)))

(event Custom|DamageResponse
  (params (DamageResponse :type E_DamageResponse%20Enum :default "NewEnumerator0") (DamageCauser :type Actor%20Object%20Reference)))

(event Custom|MC_AttachPrimary
  ;[0.15 0.15 0.15 0.5] MC Attach Primary
  (if (Variables|Weapons_Primary|GetOwnPrimaryWeapon?)
    (bind _primaryweaponbase (Variables|Weapons_Primary|GetPrimaryWeaponBase)
      (:then
        (Default|MultiStopWeaponRotation _primaryweaponbase)
        (Transformation|AttachComponentToComponent _primaryweaponbase (Variables|Character|GetMesh) (Utilities|Struct|BreakS_WeaponInfo (Variables|Weapons_Primary|GetPrimaryWeaponInfo)) "SnapToTarget" "SnapToTarget" "SnapToTarget" true)
        (CallFunction|MCCombatState (Utilities|Struct|BreakS_WeaponInfo (Variables|Weapons_Primary|GetPrimaryWeaponInfo)))
        (Variables|Weapons|SetWeaponBase (Variables|Weapons_Primary|GetPrimaryWeaponBase))
        (Variables|Weapons|SetWeaponInfo (Variables|Weapons_Primary|GetPrimaryWeaponInfo)))
      (:else))))

(event Custom|SRV_UpdatePrimaryInfo?
  (params (RowName :type Name))
  (bind _self self)
  (bind _output_get (Variables|Weapons|SetRow%20Name RowName))
  (bind _returnvalue (Utilities|GetDataTableRow "/Game/_Main/Objects/Weapons/DT_Weapons.DT_Weapons" _output_get)
    (:then
      (bind _output_get_2 (Variables|Weapons_Primary|SetOwnPrimaryWeapon? true))
      (bind _structout (Utilities|Struct|SetmembersinS_WeaponInfo _returnvalue _output_get_2))
      (bind _output_get_3 (Variables|Weapons_Primary|SetPrimaryWeaponInfo _structout))
      (bind _returnvalue_2 (Game|SpawnActorfromClass (Utilities|Struct|BreakS_WeaponInfo _output_get_3) (Transformation|GetActorTransform) "AlwaysSpawn" "MultiplyWithRoot" _self 0.0 _self))
      (bind _output_get_4 (Variables|Weapons_Primary|SetPrimaryWeaponBase _returnvalue_2))
      (Collision|SetCollisionEnabled (Variables|/Game/_Main/Objects/BP_Pickup.BP_Pickup_C|GetSphere _output_get_4) "NoCollision"))))

(event Custom|SRV_HavePrimaryWeapon?
  (params (HavePrimaryWeapon? :type Boolean) (RowName :type Name))
  (if HavePrimaryWeapon?
    (Development|PrintString "Own Primary")
    (else
      (CallFunction|SRVUpdatePrimaryInfo? RowName)
      (CallFunction|MCAttachPrimary))))

(event Custom|MC_HidePrimary
  (bind _primaryweaponinfo (Variables|Weapons_Primary|GetPrimaryWeaponInfo))
  (bind (_own_ _hiddensocket) (Utilities|Struct|BreakS_WeaponInfo _primaryweaponinfo))
  ;[0.15 0.15 0.15 0.5] MC Hide Primary
  (if _own_
    (Transformation|AttachComponentToComponent (Variables|Weapons_Primary|GetPrimaryWeaponBase) (Variables|Character|GetMesh) _hiddensocket "SnapToTarget" "SnapToTarget" "SnapToTarget" true)))

(event Custom|EquipPrimary
  (CallFunction|MCAttachPrimary))

(event Custom|MC_AttachSecondary
  ;[0.15 0.15 0.15 0.5] MC Attach Primary
  (if (Variables|Weapons_Secondary|GetOwnSecondaryWeapon)
    (bind _secondaryweaponbase (Variables|Weapons_Secondary|GetSecondaryWeaponBase)
      (:then
        (Default|MultiStopWeaponRotation _secondaryweaponbase)
        (Transformation|AttachComponentToComponent _secondaryweaponbase (Variables|Character|GetMesh) (Utilities|Struct|BreakS_WeaponInfo (Variables|Weapons_Secondary|GetSecondaryWeaponInfo)) "SnapToTarget" "SnapToTarget" "SnapToTarget" true)
        (CallFunction|MCCombatState (Utilities|Struct|BreakS_WeaponInfo (Variables|Weapons_Secondary|GetSecondaryWeaponInfo)))
        (Variables|Weapons|SetWeaponBase (Variables|Weapons_Secondary|GetSecondaryWeaponBase))
        (Variables|Weapons|SetWeaponInfo (Variables|Weapons_Secondary|GetSecondaryWeaponInfo)))
      (:else))))

(event Custom|SRV_UpdateSecondaryWeapon?
  (params (RowName :type Name))
  (bind _self self)
  (bind _output_get (Variables|Weapons|SetRow%20Name RowName))
  (bind _returnvalue (Utilities|GetDataTableRow "/Game/_Main/Objects/Weapons/DT_Weapons.DT_Weapons" _output_get)
    (:then
      (bind _output_get_2 (Variables|Weapons_Secondary|SetOwnSecondaryWeapon true))
      (bind _structout (Utilities|Struct|SetmembersinS_WeaponInfo _returnvalue _output_get_2))
      (bind _output_get_3 (Variables|Weapons_Secondary|SetSecondaryWeaponInfo _structout))
      (bind _returnvalue_2 (Game|SpawnActorfromClass (Utilities|Struct|BreakS_WeaponInfo _output_get_3) (Transformation|GetActorTransform) "AlwaysSpawn" "MultiplyWithRoot" _self 0.0 _self))
      (bind _output_get_4 (Variables|Weapons_Secondary|SetSecondaryWeaponBase _returnvalue_2))
      (Collision|SetCollisionEnabled (Variables|/Game/_Main/Objects/BP_Pickup.BP_Pickup_C|GetSphere _output_get_4) "NoCollision"))))

(event Custom|SRV_HaveSecondaryWeapon
  (params (HavePrimaryWeapon? :type Boolean) (RowName :type Name))
  (if HavePrimaryWeapon?
    (Development|PrintString "Own Secondary")
    (else
      (CallFunction|SRVUpdateSecondaryWeapon? RowName)
      (CallFunction|MCAttachSecondary))))

(event Custom|MC_HideSecondary
  (bind _secondaryweaponinfo (Variables|Weapons_Secondary|GetSecondaryWeaponInfo))
  (bind (_own_ _hiddensocket) (Utilities|Struct|BreakS_WeaponInfo _secondaryweaponinfo))
  ;[0.15 0.15 0.15 0.5] MC Hide Primary
  (if _own_
    (Transformation|AttachComponentToComponent (Variables|Weapons_Secondary|GetSecondaryWeaponBase) (Variables|Character|GetMesh) _hiddensocket "SnapToTarget" "SnapToTarget" "SnapToTarget" true)))

(event Custom|SRV_EquipSecondary
  (CallFunction|MCAttachSecondary)
  (CallFunction|MCHidePrimary))

(fn ConstructionScript
  (bind _bpc_damagesystem (Variables|Default|GetBPC_DamageSystem))
  (|CallParentFunction)
  (EventDispatchers|BindEventtoEDonDeath _bpc_damagesystem (EventDispatchers|CreateEvent :!event Custom|Death))
  (EventDispatchers|BindEventtoEDonBlocked _bpc_damagesystem (EventDispatchers|CreateEvent :!event Custom|Blocked))
  (EventDispatchers|BindEventtoOnDamageResponse _bpc_damagesystem (EventDispatchers|CreateEvent :!event Custom|DamageResponse)))

(fn FOwnWeapon
  (params (ActiveWeapon :type E_ActiveWeapon%20Enum :default "NewEnumerator0") (RowName :type Name))
  (switch Utilities|FlowControl|Switch|SwitchonE_ActiveWeapon ActiveWeapon
    (:NewEnumerator1
      (CallFunction|SRVHavePrimaryWeapon? (Variables|Weapons_Primary|GetOwnPrimaryWeapon?) RowName))
    (:NewEnumerator2
      (CallFunction|SRVHaveSecondaryWeapon (Variables|Weapons_Secondary|GetOwnSecondaryWeapon) RowName))))

(fn CharacterCombatBase
  (return self))

(fn GetCurrentHealth
  (return (Variables|/Game/_Main/Components/BPC_DamageSystem.BPC_DamageSystem_C|GetCurrentHealth (Variables|Default|GetBPC_DamageSystem))))

(fn GetMaxHealth
  (return (Variables|/Game/_Main/Components/BPC_DamageSystem.BPC_DamageSystem_C|GetMaxHealth (Variables|Default|GetBPC_DamageSystem))))

(fn Heal
  (params (Amount :type Float%20%28double-precision%29))
  (bind _currenthealth (Default|FHeal (Variables|Default|GetBPC_DamageSystem) Amount))
  (return _currenthealth))

(fn TakeDamage
  (params (DamageInfo :type S%20Damage%20Info%20Structure) (DamageCauser :type Actor%20Object%20Reference))
  (bind _wasdamaged_ (Default|FTakeDamage (Variables|Default|GetBPC_DamageSystem) DamageInfo DamageCauser))
  (return _wasdamaged_))
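; Base character Blueprint that sets up its components and handles equipping picked-up weapons.
; After a one-second delay on BeginPlay, the authority initializes the base and interact components.
; The interact component's equip event stores the pickup and calls MC_AttachPrimary to snap it to the mesh's Active_Rifle socket.
; MC_CombatState then passes a blendspace to the AnimInstance, and a CharacterBase getter returns self.
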(event OnInteractionEquip(BPC_Interact)
  (params (Equip :type BP%20Pickup%20Object%20Reference))
  ;[0.15 0.15 0.15 0.5] Interaction Equip
  (Variables|Default|SetPickup Equip)
  (CallFunction|MCAttachPrimary))

(event Custom|MC_AttachPrimary
  ;[0.15 0.15 0.15 0.5] MC Attach Primary
  (bind _pickup (Variables|Default|GetPickup)
    (:then
      (Transformation|AttachComponentToComponent _pickup (Variables|Character|GetMesh) "Active_Rifle" "SnapToTarget" "SnapToTarget" "SnapToTarget" true)
      (CallFunction|MCCombatState (Variables|Default|GetBlendspace)))
    (:else)))

(event EventBeginPlay
  ;[0.15 0.15 0.15 0.5] Event Begin Play
  (Utilities|FlowControl|Delay 1.0)
  (Networking|SwitchHasAuthority
    (:Authority
      (Default|Initialize (Variables|Default|GetBPC_Base)))))

(event Custom|MC_CombatState
  (params (Blendspace :type Integer))
  ;[0.15 0.15 0.15 0.5] MC Combat State
  (Class|BPIAnimBPPlayer|CombatState(Message) (Components|SkeletalMesh|GetAnimInstance (Variables|Character|GetMesh)) Blendspace))

(fn ConstructionScript)

(fn CharacterBase
  (return self))
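; Damage component that tracks health, armor and death for its owner, broadcasting updates, blocks, death and damage responses through event dispatchers.
; FTakeDamage uses a macro to check death, invincibility and blocking, then reduces health directly and triggers death or an interrupt response.
; Only SRV_DecreaseHealth routes damage through armor, passing the full amount to health once armor reaches zero.
; Heal and armor-increase functions clamp to maximums and work only while alive.
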(event Custom|SetInitialArmor
  (params (Value :type Float%20%28double-precision%29))
  (bind _output_get (Variables|Default|SetCurrentArmor (Math|Float|Clamp(Float) Value 0.0 (Variables|Default|GetMaxArmor))))
  (Default|CallEDUpdateArmor _output_get (Variables|Default|GetMaxArmor)))

(event Custom|SRV_DecreaseHealth
  (params (Damage :type Float%20%28double-precision%29))
  (bind _amount (CallFunction|FCheckforArmor Damage))
  (bind _output_get (Variables|Default|SetCurrentHealth (Math|Float|Clamp(Float) (- (Variables|Default|GetCurrentHealth) _amount) 0.0 (Variables|Default|GetMaxHealth))))
  (Default|CallEDUpdateHealth _output_get (Variables|Default|GetMaxHealth)))

(event Custom|SetInitialHealth
  (params (Value :type Float%20%28double-precision%29))
  ;[0.15 0.15 0.15 0.5] SetInitialHealth
  (bind _output_get (Variables|Default|SetCurrentHealth (Math|Float|Clamp(Float) Value 0.0 (Variables|Default|GetMaxHealth))))
  (Default|CallEDUpdateHealth _output_get (Variables|Default|GetMaxHealth)))

(event EventLoadComponent
  (CallFunction|SetInitialHealth (Variables|Default|GetMaxHealth))
  (CallFunction|SetInitialArmor (Variables|Default|GetMaxArmor)))

(fn FTakeDamage
  (params (S_DamageInfo :type S%20Damage%20Info%20Structure%20%28by%20ref%29) (DamageCauser :type Actor%20Object%20Reference))
  (bind (_amount _damagetype _damageresponse _shoulddamageinvincible_ _canbeblocked_ _canbeparried_ _forceinterrupt_) (Utilities|Struct|BreakS_DamageInfo S_DamageInfo))
  (Utilities|MCanbeDamaged _shoulddamageinvincible_ _canbeblocked_
    (:BlockDamage
      (Default|CallEDonBlocked _canbeparried_)
      (return false))
    (:DoDamage
      (bind _output_get (Variables|Default|SetCurrentHealth (Math|Float|Clamp(Float) (- (Variables|Default|GetCurrentHealth) _amount) 0.0 (Variables|Default|GetMaxHealth))))
      (Default|CallEDUpdateHealth (Variables|Default|GetCurrentHealth) (Variables|Default|GetMaxHealth))
      (if (<= _output_get 0.0)
        (if (not (Variables|Default|GetIsDead?))
          (Variables|Default|SetIsDead? true)
          (Default|CallEDonDeath DamageCauser)
          (return true))
        (elif (or (Variables|Default|GetIsInterruptable?) _forceinterrupt_)
          (Default|CallOnDamageResponse _damageresponse DamageCauser)
          (return true))))
    (:NoDamage
      (return false))))

(fn FHeal
  (params (Amount :type Float%20%28double-precision%29))
  (if (not (Variables|Default|GetIsDead?))
    (bind _output_get (Variables|Default|SetCurrentHealth (Math|Float|Clamp(Float) (+ Amount (Variables|Default|GetCurrentHealth)) 0.0 (Variables|Default|GetMaxHealth))))
    (Default|CallEDUpdateHealth _output_get (Variables|Default|GetMaxHealth))
    (return _output_get)))

(fn FCheckforArmor
  (params (Damage :type Float%20%28double-precision%29))
  (bind _output_get (Variables|Default|SetCurrentArmor (Math|Float|Clamp(Float) (- (Variables|Default|GetCurrentArmor) Damage) 0.0 (Variables|Default|GetMaxArmor))))
  (Default|CallEDUpdateArmor _output_get (Variables|Default|GetMaxArmor))
  (if (<= (Variables|Default|GetCurrentArmor) 0.0)
    (return Damage)))

(fn FIncreaseArmor
  (params (Amount :type Float%20%28double-precision%29))
  (if (not (Variables|Default|GetIsDead?))
    (bind _output_get (Variables|Default|SetCurrentArmor (Math|Float|Clamp(Float) (+ Amount (Variables|Default|GetCurrentArmor)) 0.0 (Variables|Default|GetMaxArmor))))
    (Default|CallEDUpdateArmor _output_get (Variables|Default|GetMaxArmor))))
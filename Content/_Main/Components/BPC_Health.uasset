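; Health component that tracks a current health value against a maximum.
; LoadComponent initializes current health to MaxHealth through SetInitialHealth, while SRV-prefixed events decrease or increase it by a given amount.
; Every change clamps the result between zero and MaxHealth, then calls the EDHealth dispatcher with current and maximum health.
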(event Custom|SetInitialHealth
  (params (Value :type Float%20%28double-precision%29))
  ;[0.15 0.15 0.15 0.5] SetInitialHealth
  (bind _output_get (Variables|Default|SetCurrentHealth (Math|Float|Clamp(Float) Value 0.0 (Variables|Default|GetMaxHealth))))
  (Default|CallEDHealth _output_get (Variables|Default|GetMaxHealth)))

(event Custom|SRV_IncreaseHealth
  (params (Damage :type Float%20%28double-precision%29))
  (bind _output_get (Variables|Default|SetCurrentHealth (Math|Float|Clamp(Float) (+ (Variables|Default|GetCurrentHealth) Damage) 0.0 (Variables|Default|GetMaxHealth))))
  (Default|CallEDHealth _output_get (Variables|Default|GetMaxHealth)))

(event Custom|SRV_DecreaseHealth
  (params (Damage :type Float%20%28double-precision%29))
  (bind _output_get (Variables|Default|SetCurrentHealth (Math|Float|Clamp(Float) (- (Variables|Default|GetCurrentHealth) Damage) 0.0 (Variables|Default|GetMaxHealth))))
  (Default|CallEDHealth _output_get (Variables|Default|GetMaxHealth)))

(event EventLoadComponent
  (CallFunction|SetInitialHealth (Variables|Default|GetMaxHealth)))
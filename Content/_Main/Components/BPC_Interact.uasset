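; Character interaction component that lets the owner equip, pick up, hold, tap or press actors implementing BPI_Interactable.
; Capsule overlaps maintain an in-range list whose last entry is active, showing a screen-space prompt or, for Pickup types, triggering interaction immediately.
; IA_Interact input goes to SRV events that branch on interaction type, while Client events update the prompt and hold/tap progress.
; Hold completion is detected in the client widget update, which then calls SRV_Interact.
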(event Custom|HandleCapsuleOverlapBegin
  (params (OverlappedComponent :type Primitive%20Component%20Object%20Reference) (OtherActor :type Actor%20Object%20Reference) (OtherComp :type Primitive%20Component%20Object%20Reference) (OtherBodyIndex :type Integer) (bFromSweep :type Boolean) (SweepResult :type Hit%20Result%20Structure%20%28by%20ref%29))
  ;[0.15 0.15 0.15 0.5] Handle Capsule Overlap Begin
  (if (Utilities|DoesObjectImplementInterface OtherActor "/Game/_Main/Systems/Interaction/BPI_Interactable.BPI_Interactable_C")
    (Utilities|Array|AddUnique (Variables|Default|GetInteractableInRange) OtherActor)
    (bind _interactiontype (Class|BPIInteractable|GetInteractionType(Message) OtherActor))
    (switch Utilities|FlowControl|Switch|SwitchonE_InteractionType _interactiontype
      (:NewEnumerator4
        (CallFunction|FRenderInteractionWidget :!label _label))
      (:NewEnumerator0
        (CallFunction|SRVInteractBegin))
      (:NewEnumerator1
        (goto _label))
      (:NewEnumerator2
        (goto _label))
      (:NewEnumerator3
        (goto _label)))))

(event Custom|HandleCapsuleOverlapEnd
  (params (OverlappedComponent :type Primitive%20Component%20Object%20Reference) (OtherActor :type Actor%20Object%20Reference) (OtherComp :type Primitive%20Component%20Object%20Reference) (OtherBodyIndex :type Integer))
  ;[0.15 0.15 0.15 0.5] Handle Capsule Overlap End
  (if (Utilities|DoesObjectImplementInterface OtherActor "/Game/_Main/Systems/Interaction/BPI_Interactable.BPI_Interactable_C")
    (Utilities|Array|RemoveItem (Variables|Default|GetInteractableInRange) OtherActor)
    (CallFunction|FRenderInteractionWidget)
    (CallFunction|FResetInteractiveState)))

(event Custom|SRV_Interact
  (bind _activeinteractable (CallFunction|FGetActiveInteractable))
  ;[0.15 0.15 0.15 0.5] SRV Interact
  (Class|BPIInteractable|Interact(Message) _activeinteractable (Variables|Default|GetCharacter%20Base))
  (CallFunction|FResetInteractiveState)
  (CallFunction|ClientSetWCInteractHidden)
  (bind _duration (Class|BPIInteractable|GetHoldDuration(Message) _activeinteractable))
  (Utilities|FlowControl|Delay _duration)
  (CallFunction|FRenderInteractionWidget)
  (CallFunction|ClientSetWCInteractVisible))

(event Custom|SRV_InteractBegin
  (bind _activeinteractable (CallFunction|FGetActiveInteractable))
  ;[0.15 0.15 0.15 0.5] SRV Interact Begin
  (Utilities|IsValid _activeinteractable
    (:Is%20Valid
      (bind _interactiontype (Class|BPIInteractable|GetInteractionType(Message) _activeinteractable))
      (switch Utilities|FlowControl|Switch|SwitchonE_InteractionType _interactiontype
        (:NewEnumerator4
          (CallFunction|SRVEquip _activeinteractable))
        (:NewEnumerator0
          (CallFunction|SRVPickup _activeinteractable))
        (:NewEnumerator1
          (CallFunction|Hold))
        (:NewEnumerator2
          (CallFunction|ClientInteractionTap))
        (:NewEnumerator3
          (CallFunction|SRVInteract))))
    (:Is%20Not%20Valid
      (Development|PrintString "InteractionBeginFailed"))))

(event EventLoadComponent
  (bind _character_base (Variables|Default|GetCharacter%20Base))
  (bind _capsulecomponent (Variables|/Script/Engine.Character|GetCapsuleComponent _character_base))
  ;[0.15 0.15 0.15 0.5] Load Component
  (Collision|BindEventtoOnComponentBeginOverlap _capsulecomponent (EventDispatchers|CreateEvent :!event Custom|HandleCapsuleOverlapBegin))
  (Collision|BindEventtoOnComponentEndOverlap _capsulecomponent (EventDispatchers|CreateEvent :!event Custom|HandleCapsuleOverlapEnd))
  (CallFunction|MCCreateWidgetComponent))

(event Custom|MC_CreateWidgetComponent
  ;[0.15 0.15 0.15 0.5] MC Create Widget Component
  (bind _returnvalue (Game|AddComponentbyClass (Components|GetOwner) "/Script/UMG.WidgetComponent" true))
  (Class|WidgetComponent|SetWidgetSpace _returnvalue "Screen")
  (Class|WidgetComponent|SetDrawSize _returnvalue "(X=250.000000,Y=30.000000)")
  (Variables|Default|SetWC_Interact _returnvalue))

(event Custom|Client_AddWidget
  (params (OwningPlayer :type Player%20Controller%20Object%20Reference) (NewLocation :type Vector) (InteractionType :type E_InteractionType%20Enum :default "NewEnumerator0"))
  ;[0.15 0.15 0.15 0.5] Client Add Widget
  (bind _returnvalue (UserInterface|CreateWidget "/Game/_Main/Systems/Interaction/W_Interact.W_Interact_C" OwningPlayer InteractionType))
  (bind _output_get (Variables|Default|SetW_Interact _returnvalue))
  (bind _wc_interact (Variables|Default|GetWC_Interact)
    (:then
      (UserInterface|SetWidget _wc_interact _output_get)
      (Transformation|SetWorldLocation _wc_interact NewLocation false false))
    (:else)))

(event Custom|Client_RemoveWidget
  ;[0.15 0.15 0.15 0.5] Client Remote Widget
  (bind _wc_interact (Variables|Default|GetWC_Interact)
    (:then
      (UserInterface|SetWidget _wc_interact 0))
    (:else)))

(event Custom|Client_SetWC_InteractVisible
  ;[0.15 0.15 0.15 0.5] Set_WC_Interact Visible
  (Rendering|SetVisibility (Variables|Default|GetWC_Interact) true false))

(event Custom|Client_SetWC_InteractHidden
  ;[0.15 0.15 0.15 0.5] Set WC_Interact Hidden
  (Rendering|SetVisibility (Variables|Default|GetWC_Interact) false false))

(event Input|EnhancedActionEvents|EnhancedInputActionIA_Interact
  (params (ActionValue :type Boolean) (ElapsedSeconds :type Float%20%28double-precision%29) (TriggeredSeconds :type Float%20%28double-precision%29) (InputAction :type Input%20Action%20Object%20Reference :default "/Game/_Main/Characters/Player/Inputs/InputActions/IA_Interact.IA_Interact"))
  ;[0.15 0.15 0.15 0.5] IA Interact
  (:Started
    (CallFunction|SRVInteractBegin))
  (:Ongoing
    (CallFunction|SRVonInteractionHold ElapsedSeconds))
  (:Canceled
    (CallFunction|SRVEndHold :!label _label))
  (:Completed
    (goto _label)))

(event Custom|SRV_Equip
  (params (Pickup :type Actor%20Object%20Reference))
  ;[0.15 0.15 0.15 0.5] SRV Equip
  (bind _pickup (Class|BPIPickup|Pickup(Message) Pickup))
  (Utilities|Array|RemoveItem (Variables|Default|GetInteractableInRange) _pickup)
  (CallFunction|CLientRemoveWidget)
  (Default|CallOnInteraction _pickup))

(event Custom|SRV_OnHoldOngoing
  (params (ElapsedSeconds :type Float%20%28double-precision%29))
  (bind _activeinteractable (CallFunction|FGetActiveInteractable))
  ;[0.15 0.15 0.15 0.5] SRV On Hold Ongoing
  (Utilities|IsValid _activeinteractable
    (:Is%20Valid
      (bind _duration (Class|BPIInteractable|GetHoldDuration(Message) _activeinteractable))
      (CallFunction|ClientUpdateHoldWidget ElapsedSeconds _duration))))

(event Custom|SRV_OnHoldEneded
  ;[0.15 0.15 0.15 0.5] SRV On Hold Ended
  (Default|CallOnHoldEnded))

(event Custom|SRV_OnInteractionHold
  (params (ElapsedSeconds :type Float%20%28double-precision%29))
  ;[0.15 0.15 0.15 0.5] SRV On  Interaction Hold
  (Default|CallOnInteractionHold ElapsedSeconds))

(event Custom|Client_UpdateHoldWidget
  (params (ElapsedSeconds :type Float%20%28double-precision%29) (Duration :type Float%20%28double-precision%29))
  ;[0.15 0.15 0.15 0.5] Client Update Hold Widget
  (bind _w_interact (Variables|Default|GetW_Interact)
    (:then
      (Default|FSetProgressPercent _w_interact (/ ElapsedSeconds Duration)))
    (:else
      _))
  (if (> ElapsedSeconds Duration)
    (CallFunction|SRVInteract)
    (CallFunction|FResetInteractiveState)))

(event Custom|SRV_EndHold
  (bind _activeinteractable (CallFunction|FGetActiveInteractable))
  ;[0.15 0.15 0.15 0.5] SRV End Hold
  (Utilities|IsValid _activeinteractable
    (:Is%20Valid
      (bind _interactiontype (Class|BPIInteractable|GetInteractionType(Message) _activeinteractable))
      (switch Utilities|FlowControl|Switch|SwitchonE_InteractionType _interactiontype
        (:NewEnumerator1
          (CallFunction|SRVonHoldEneded)
          (EventDispatchers|UnbindallEventsfromOnInteractionHold))))))

(event Custom|Client_ResetWidgetProgress
  ;[0.15 0.15 0.15 0.5] Client Reset Widget Progress
  (bind _w_interact (Variables|Default|GetW_Interact)
    (:then
      (Default|FSetProgressPercent _w_interact 0.0)
      (EventDispatchers|UnbindEventfromOnHoldEnded (delegate Custom|Client_ResetWidgetProgress)))
    (:else)))

(event Custom|Hold
  ;[0.15 0.15 0.15 0.5] Hold
  (EventDispatchers|BindEventtoOnInteractionHold (EventDispatchers|CreateEvent :!event Custom|SRV_OnHoldOngoing))
  (EventDispatchers|BindEventtoOnHoldEnded (delegate Custom|Client_ResetWidgetProgress)))

(event Custom|Client_TapWidget
  (params (InPercent :type Float%20%28single-precision%29))
  ;[0.15 0.15 0.15 0.5] Client Tap Widget
  (bind _w_interact (Variables|Default|GetW_Interact)
    (:then
      (Default|FSetProgressPercent _w_interact InPercent))
    (:else)))

(event Custom|SRV_TapMain
  ;[0.15 0.15 0.15 0.5] SRV Tap Main
  (Math|Integer|IncrementInt (Variables|Default|GetCurrentTapCount)
    (:%20%20
      (bind _tapcount (Class|BPIInteractable|GetTapCount(Message) (CallFunction|FGetActiveInteractable)))
      (if (<= _tapcount 0)
        (CallFunction|SRVInteract)
        (else
          (CallFunction|ClientTapWidget (/ (Variables|Default|GetCurrentTapCount) _tapcount))
          (if (>= (Variables|Default|GetCurrentTapCount) _tapcount)
            (CallFunction|SRVInteract)))))))

(event Custom|Client_InteractionTap
  ;[0.15 0.15 0.15 0.5] Client Interaction Tap
  (Audio|PlaySoundatLocation "/Engine/VREditor/Sounds/UI/Teleport_Committed.Teleport_Committed" (Transformation|GetActorLocation (Components|GetOwner)) "0, 0, 0" 1.0 1.0 0.0 0 0 0 0)
  (CallFunction|SRVTapMain))

(event Custom|SRV_Pickup
  (params (Actor :type Actor%20Object%20Reference))
  ;[0.15 0.15 0.15 0.5] SRV Pickup
  (bind _pickup (Class|BPIPickup|Pickup(Message) Actor))
  (Utilities|Array|RemoveItem (Variables|Default|GetInteractableInRange) _pickup)
  (CallFunction|ClientRemoveWidget)
  (Default|CallOnInteraction _pickup)
  (Development|PrintString (Utilities|GetDisplayName _pickup)))

(fn FGetActiveInteractable
  (bind _interactableinrange (Variables|Default|GetInteractableInRange))
  (return (Utilities|Array|Get(acopy) _interactableinrange (Utilities|Array|LastIndex _interactableinrange))))

(fn FRenderInteractionWidget
  (bind _activeinteractable (CallFunction|FGetActiveInteractable))
  (Utilities|IsValid _activeinteractable
    (:Is%20Valid
      (bind _interactiontype (Class|BPIInteractable|GetInteractionType(Message) _activeinteractable))
      (CallFunction|ClientAddWidget (Game|GetPlayerController 0) (CallFunction|FGetActiveInteractableLocation) _interactiontype))
    (:Is%20Not%20Valid
      (CallFunction|CLientRemoveWidget)))
  (return))

(fn FGetActiveInteractableLocation
  (bind _activeinteractable (CallFunction|FGetActiveInteractable))
  (Utilities|IsValid _activeinteractable
    (:Is%20Valid
      (bind _location (Class|BPIInteractable|GetInteractLocation(Message) _activeinteractable))
      (return (Math|Vector|SelectVector (Transformation|GetActorLocation _activeinteractable) _location (Math|Vector|VectorIsZero _location))))))

(fn FResetInteractiveState
  (EventDispatchers|UnbindEventfromOnInteractionHold (EventDispatchers|CreateEvent :!event Custom|SRV_OnHoldOngoing))
  (Variables|Default|SetCurrentTapCount 0)
  (CallFunction|FRenderInteractionWidget)
  (return))
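; Actor component that tracks an armor pool, holding current armor between zero and a maximum.
; LoadComponent fills armor to the maximum through InitialArmor, while SRV-prefixed events increase it or reduce it by incoming damage.
; Every change is clamped and then broadcast through the EDArmor event dispatcher with the current and maximum values.
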(event Custom|InitialArmor
  (params (Armor :type Float%20%28double-precision%29))
  ;[0.15 0.15 0.15 0.5] Initial Armor
  (bind _output_get (Variables|Default|SetCurrentArmor (Math|Float|Clamp(Float) Armor 0.0 (Variables|Default|GetMaxArmor))))
  (Default|CallEDArmor _output_get (Variables|Default|GetMaxArmor)))

(event Custom|SRV_IncreaseArmor
  (params (Armor :type Float%20%28double-precision%29))
  ;[0.15 0.15 0.15 0.5] Increase Armor
  (bind _output_get (Variables|Default|SetCurrentArmor (Math|Float|Clamp(Float) (+ (Variables|Default|GetCurrentArmor) Armor) 0.0 (Variables|Default|GetMaxArmor))))
  (Default|CallEDArmor _output_get (Variables|Default|GetMaxArmor)))

(event Custom|SRV_DecreaseArmor
  (params (Damage :type Float%20%28double-precision%29))
  ;[0.15 0.15 0.15 0.5] Decrease Armor
  (bind _output_get (Variables|Default|SetCurrentArmor (Math|Float|Clamp(Float) (- (Variables|Default|GetCurrentArmor) Damage) 0.0 (Variables|Default|GetMaxArmor))))
  (Default|CallEDArmor _output_get (Variables|Default|GetMaxArmor)))

(event EventLoadComponent
  (CallFunction|InitialArmor (Variables|Default|GetMaxArmor)))
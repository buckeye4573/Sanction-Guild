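; Actor component that implements an object pool, pre-spawning actors of a configurable class for reuse.
; Shortly after BeginPlay it spawns the pool, passing each actor a TimeToLive and marking it not in use.
; Spawn requests linearly search for the first free actor, move it to the requested transform and mark it in use.
; When none is free it prints a failure message rather than growing the pool.
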(event Custom|InitializedPool
  (params (Class :type BP%20Pooled%20Actor%20Class%20Reference))
  ;[0.15 0.15 0.15 0.5] Initialized Pool
  (for _index (range 0 (Variables|Default|GetPoolSize))
    (bind _returnvalue (Game|SpawnActorfromClass Class (Math|Transform|MakeTransform "0, 0, 0" "0, 0, 0" "1.000000,1.000000,1.000000") "Undefined" "MultiplyWithRoot" 0 (Variables|Default|GetTime%20to%20Live) 0))
    (Utilities|Array|AddUnique (Variables|Default|GetObjectPool) _returnvalue)
    (Default|SetinUse _returnvalue false)))

(event EventBeginPlay
  ;[0.15 0.15 0.15 0.5] Event Begin Play
  (Utilities|FlowControl|Delay 0.2)
  (CallFunction|InitializedPool (Variables|Default|GetPooledActorClass)))

(fn FFindFirstAvailableActor
  (for _array_element (Variables|Default|GetObjectPool)
    (if (not (Variables|/Game/_Main/Patterns/Pool/BP_PooledActor.BP_PooledActor_C|GetInUse _array_element))
      (return _array_element))))

(fn FSpawnfromPool
  (params (SpawnTransform :type Transform))
  (bind _pooledactor (CallFunction|FFindFirstAvailableActor))
  (Utilities|IsValid _pooledactor
    (:Is%20Valid
      (Transformation|SetActorTransform _pooledactor SpawnTransform)
      (Default|SetinUse _pooledactor true)
      (return _pooledactor))
    (:Is%20Not%20Valid
      (Development|PrintString "Failed To Spawn Actor From Pool"))))
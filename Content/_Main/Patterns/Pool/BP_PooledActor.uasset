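; BP_PooledActor is an actor for object pooling that is switched on and off for reuse.
; SetInUse stores the in-use flag, toggles collision, visibility and tick to match, and clears the time-to-live timer.
; ReturnToPool deactivates the actor through SetInUse, while SRV_RespawnObject reactivates it after a TimeToLive delay.
; SRV_DespawnObject starts a TimeToLive timer and stores its handle.
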(event Custom|SetInUse
  (params (InUse? :type Boolean))
  ;[0.15 0.15 0.15 0.5] Set In Use
  (bind _output_get (Variables|Default|SetInUse InUse?))
  (Collision|SetActorEnableCollision _output_get)
  (Rendering|SetActorHiddenInGame (not _output_get))
  (Actor|Tick|SetActorTickEnabled _output_get)
  (Utilities|Time|ClearandInvalidateTimerbyHandle (Variables|Default|GetTimeToLiveTimer))
  (if _output_get
    _))

(event Custom|ReturnToPool
  ;[0.15 0.15 0.15 0.5] Return To Pool
  (CallFunction|SetinUse false))

(event Custom|SRV_RespawnObject
  ;[0.15 0.15 0.15 0.5] Respawn
  (Utilities|FlowControl|Delay (Variables|Default|GetTimeToLive))
  (CallFunction|SetinUse true))

(event Custom|SRV_DespawnObject
  ;[0.15 0.15 0.15 0.5] Despawn
  (bind _returnvalue (Utilities|Time|SetTimerbyEvent (EventDispatchers|CreateEvent :!event Custom|ReturnToPool) (Variables|Default|GetTimeToLive)))
  (Variables|Default|SetTimeToLiveTimer _returnvalue))

(event EventBeginPlay
  ;[0.15 0.15 0.15 0.5] Event Begin Play
)

(fn ConstructionScript)